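; Character component that handles player farming: planting selected DT_Farmables seeds on Growing_Plot actors and interacting with plants.
; Camera traces target plants for water, fertilizer, cure, sickness, damage and interaction, intended to run on the server.
; RepNotifies drive demo hand props and montages, using a play counter so repeated animations still fire.
; On BeginPlay, the server respawns non-hand-placed plants from the FarmSave slot and relinks pluckable yields by GUID.
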(event Custom|Event:%20Try%20Apply%20Damage
  ;[0.07888 1 0] All interactions with the plants. All logic is done on the server
  (bind _hitactor (CallFunction|Trace "TraceTypeQuery3"))
  (bind _asplayer_controller (Utilities|Casting|CastToPlayerController (Pawn|GetController (Variables|Default|GetOwning%20character%20referemce))))
  (Game|Damage|ApplyDamage _hitactor 25.0 0 _asplayer_controller)
  (CallFunction|PlayAnimation "/Game/ResourcePack/Animations/Melee/Anim_swing_sword_sidewards.Anim_swing_sword_sidewards")
  (CallFunction|SpawnMesh "/Game/ResourcePack/Weapons/Swords/SM_Sword_Steel.SM_Sword_Steel"))

(event Custom|Play%20Animation
  (params (Animation%20to%20play :type Anim%20Sequence%20Base%20Object%20Reference))
  ;[1 1 1] For show, an animation and mesh showing. In your own system you will want to equip items, and show your animation integrated in your own framework
  ;;[1 1 1] Play a dynamic animation montage.
  ;; Network peformance wise you do not want to use a multicast but want to replicate the action from server to client.
  ;; Rep Notifies are only triggered if the variables are changed. That is why we use a workarround to play each animation via notify of the animation amounts played (always an unique number and therefore notified)
  ;; In Unreal the notofication runs as well on the server as on the clients (in replication radius)
  (Variables|Default|SetAnimation%20To%20Play Animation%20to%20play)
  (Variables|Default|SetAmount%20of%20animations%20played (+ (Variables|Default|GetAmount%20of%20animations%20played) 1)))

(event Custom|Spawn_Mesh
  (params (Mesh :type Static%20Mesh%20Object%20Reference))
  ;[1 1 1] For show, an animation and mesh showing. In your own system you will want to equip items, and show your animation integrated in your own framework
  ;;[1 1 1] Show a mesh for 2 second.
  (Utilities|IsValid (Variables|Default|GetCurrent%20%20Equiped%20Mesh)
    (:Is%20Valid
      (if (not (== (Variables|Default|GetCurrent%20%20Equiped%20Mesh) Mesh))
        (Variables|Default|SetCurrent%20%20Equiped%20Mesh 0)
        (Variables|Default|SetCurrent%20%20Equiped%20Mesh Mesh :!label _label)
        (Utilities|FlowControl|Delay 5.0)
        (Variables|Default|SetCurrent%20%20Equiped%20Mesh 0)))
    (:Is%20Not%20Valid
      (goto _label))))

(event Custom|Event%20Select%20farmable%20up%20down
  ;[1 1 1] Scroll through the datatable items for preview placement.  Can be deleted in own project if you implement own selection method. Tip: My building system has a radial many for selection
  (Variables|Default|SetCurrent%20selected%20row (Math|Integer|Clamp(Integer) (- (Variables|Default|GetCurrent%20selected%20row) 1) 0 (Utilities|Array|Length (Variables|Default|GetData%20Table%20Rows)))))

(event Custom|Event%20Select%20farmable%20up
  ;[1 1 1] Scroll through the datatable items for preview placement.  Can be deleted in own project if you implement own selection method. Tip: My building system has a radial many for selection
  (Variables|Default|SetCurrent%20selected%20row (Math|Integer|Clamp(Integer) (+ (Variables|Default|GetCurrent%20selected%20row) 1) 0 (Utilities|Array|Length (Variables|Default|GetData%20Table%20Rows)))))

(event Custom|Event:%20Spawn%20Seed
  (params (SpawnTransform :type Transform) (Plant :type Data%20Table%20Row%20Handle%20Structure%20%28by%20ref%29))
  (bind (_datatable _rowname) (Utilities|Struct|BreakDataTableRowHandle Plant))
  ;[1 1 1] Spawn Seed
  (bind _returnvalue (Utilities|GetDataTableRow _datatable _rowname)
    (:then
      ;;[1 1 1] Spawn the specific actor(plant type)
      (bind _asbp_farming_master (Utilities|Casting|CastToBP_Farming_MasterClass (Utilities|Struct|BreakStruct_PlantAttributes_Generic (Utilities|Struct|BreakStruct_Plant _returnvalue))))
      (Game|SpawnActorfromClass _asbp_farming_master SpawnTransform "AlwaysSpawn" 0 0.0 0 0.0 Plant false false false 1e+02 "" 0.0 0.0 0.0 false false false 0.0 0 false false false true 0))))

(event Custom|Load%20Farming
  ;[1 1 1] spawn from save if server and we only want to do it once, so only character 0 excecutes this function
  (if (and (Networking|IsServer) (Class|Pawn|IsControlled (Variables|Default|GetOwning%20character%20referemce)))
    (Utilities|IsValid (Game|GetPlayerCharacter 0) :!label _label
      (:Is%20Valid
        (CallFunction|Event:SpawnPlantsfromSave)))
    (elif (Networking|IsDedicatedServer)
      (goto _label))))

(event Custom|Spawn%20Seed%20on%20trace%20location
  ;[1 1 1] Spawn Seed
  (bind (_hitactor _hitcomponent _hit _outhit) (CallFunction|Trace "TraceTypeQuery1"))
  (if _hit
    ;;[1 1 1] Only place when looked at actor is growning plot
    (if (Actor|ActorHasTag _hitactor "Growing_Plot")
      (CallFunction|Event:SpawnSeed (Math|Transform|MakeTransform (.Location (Collision|BreakHitResult _outhit)) "0, 0, 0" "1,1,1") (Utilities|Struct|MakeDataTableRowHandle "/Game/FarmingSystem/Datamodel/DT_Farmables.DT_Farmables" (Utilities|Array|Get(acopy) (Variables|Default|GetData%20Table%20Rows) (Variables|Default|GetCurrent%20selected%20row)))))))

(event Custom|Event:%20Try%20add%20Fertilizer
  ;[0.07888 1 0] All interactions with the plants. All logic is done on the server
  (bind _hitactor (CallFunction|Trace "TraceTypeQuery3"))
  (bind _asplayer_controller (Utilities|Casting|CastToPlayerController (Pawn|GetController (Variables|Default|GetOwning%20character%20referemce))))
  (Class|BPIFarming|TryAddFertilizer(Message) _hitactor 25.0 _asplayer_controller)
  (CallFunction|PlayAnimation "/Game/ResourcePack/Animations/State_Animations/Anim_grab.Anim_grab")
  (CallFunction|SpawnMesh "/Game/ResourcePack/Raw_Resources/Open_Sack/Meshes/SM_Open_Sack_Fertilizer_Small.SM_Open_Sack_Fertilizer_Small"))

(event Custom|Event:%20Try%20add%20Water
  ;[0.07888 1 0] All interactions with the plants. All logic is done on the server
  (bind _hitactor (CallFunction|Trace "TraceTypeQuery3"))
  (bind _asplayer_controller (Utilities|Casting|CastToPlayerController (Pawn|GetController (Variables|Default|GetOwning%20character%20referemce))))
  (Class|BPIFarming|TryAddWater(Message) _hitactor 25.0 _asplayer_controller)
  (CallFunction|PlayAnimation "/Game/ResourcePack/Animations/State_Animations/Anim_grab.Anim_grab")
  (CallFunction|SpawnMesh "/Game/ResourcePack/Tools/Watering_Can/SM_Watering_Can.SM_Watering_Can"))

(event Custom|Event:%20Interact
  ;[0.07888 1 0] All interactions with the plants. All logic is done on the server
  (bind _hitactor (CallFunction|Trace "TraceTypeQuery3"))
  (bind _asplayer_controller (Utilities|Casting|CastToPlayerController (Pawn|GetController (Variables|Default|GetOwning%20character%20referemce))))
  (Class|BPIFarming|Interact(Message) _hitactor _asplayer_controller)
  (CallFunction|PlayAnimation "/Game/ResourcePack/Animations/State_Animations/Anim_grab.Anim_grab")
  (CallFunction|SpawnMesh "/Game/ResourcePack/Props/Basket/Mesh/SM_Basket_Small.SM_Basket_Small"))

(event Custom|Event:%20Try%20Cure%20Plant
  ;[0.07888 1 0] All interactions with the plants. All logic is done on the server
  (bind _hitactor (CallFunction|Trace "TraceTypeQuery3"))
  (bind _asplayer_controller (Utilities|Casting|CastToPlayerController (Pawn|GetController (Variables|Default|GetOwning%20character%20referemce))))
  (Class|BPIFarming|TryCurePlant(Message) _hitactor _asplayer_controller)
  (CallFunction|PlayAnimation "/Game/ResourcePack/Animations/State_Animations/Anim_grab.Anim_grab")
  (CallFunction|SpawnMesh "/Game/ResourcePack/Tools/Bucket/Mesh/SM_Bucket.SM_Bucket"))

(event Custom|Event:%20Set%20plant%20to%20sick
  ;[0.07888 1 0] All interactions with the plants. All logic is done on the server
  (bind _hitactor (CallFunction|Trace "TraceTypeQuery3"))
  (bind _asbp_farming_master (Utilities|Casting|CastToBP_Farming_Master _hitactor))
  (Default|Event:SwitchPlantSickness _asbp_farming_master true)
  (CallFunction|PlayAnimation "/Game/ResourcePack/Animations/State_Animations/Anim_grab.Anim_grab"))

(event Custom|Event:%20Spawn%20Plants%20from%20save
  ;[1 1 1] spawn from save if server and we only want to do it once, so only character 0 excecutes this function
  (CallFunction|SpawnPlantsfromSave))

(event Custom|Save%20Data%20Table%20row%20names%20for%20preview%20selection
  ;[1 1 1] Scroll through the datatable items for preview placement.  Can be deleted in own project if you implement own selection method. Tip: My building system has a radial many for selection
  (bind _outrownames (DataTable|GetDataTableRowNames "/Game/FarmingSystem/Datamodel/DT_Farmables.DT_Farmables"))
  (Variables|Default|SetData%20Table%20Rows _outrownames))

(event EventBeginPlay
  (Utilities|FlowControl|Sequence
    (:then_0
      ;[1 1 1] Store character and camera reference
      (bind _ascharacter (Utilities|Casting|CastToCharacter (Components|GetOwner)))
      (bind _output_get (Variables|Default|SetOwning%20character%20referemce _ascharacter))
      (Variables|Default|SetCamera%20Reference (Actor|GetComponentbyClass _output_get "/Script/Engine.CameraComponent")))
    (:then_1
      ;[1 1 1] Load farming
      (CallFunction|LoadFarming))
    (:then_2
      ;[1 1 1] Save data table row names. Can be deleted in own project if you implement own selection method. Tip: My building system has a radial many for selection
      (CallFunction|SaveDataTableRowNamesforPreviewSelection))))

(fn Trace
  (params (TraceChannel :type ETraceTypeQuery%20Enum :default "TraceTypeQuery1"))
  (bind _camera_reference (Variables|Default|GetCamera%20Reference))
  (bind _returnvalue (Transformation|GetWorldLocation _camera_reference))
  (bind _returnvalue_2 (Math|Vector|GetForwardVector _camera_reference))
  ;[1 1 1] Trace from camera. Used for multiple purposes throughout the sytem
  (bind (_outhit _returnvalue_3) (Collision|LineTraceByChannel (+ _returnvalue (* _returnvalue_2 2.5e+02)) (+ _returnvalue (* _returnvalue_2 1e+03)) TraceChannel false 0 "None"))
  (return (.HitActor (Collision|BreakHitResult _outhit)) (.HitComponent (Collision|BreakHitResult _outhit)) _returnvalue_3 _outhit))

(fn SpawnPlantsfromSave
  (bind _returnvalue (SaveGame|DoesSaveGameExist "FarmSave"))
  (if _returnvalue
    (bind _returnvalue_2 (SaveGame|LoadGamefromSlot "FarmSave"))
    (bind _asbp_save_plants (Utilities|Casting|CastToBP_Save_Plants _returnvalue_2))
    (LocalVariables|SetLocal%20Save _asbp_save_plants)
    (for _array_element (Variables|/Game/FarmingSystem/Save/BP_Save_Plants.BP_Save_Plants_C|GetPlants _asbp_save_plants)
      (if (not (.IsManuallyplacedinworld (Utilities|Struct|BreakStruct_Saved_Plants _array_element)))
        (bind _asbp_farming_master (Utilities|Casting|CastToBP_Farming_MasterClass (.Actor (Utilities|Struct|BreakStruct_Saved_Plants _array_element))))
        (bind _returnvalue_3 (Game|SpawnActorfromClass _asbp_farming_master (.Transform (Utilities|Struct|BreakStruct_Saved_Plants _array_element)) "AlwaysSpawn" 0 (.Current_Growth_Time (Utilities|Struct|BreakStruct_Saved_Plants _array_element)) (.Current_Growth_Stage (Utilities|Struct|BreakStruct_Saved_Plants _array_element)) (.Current_Growth_Percentage (Utilities|Struct|BreakStruct_Saved_Plants _array_element)) (.PlantDataTableRow (Utilities|Struct|BreakStruct_Saved_Plants _array_element)) (.Can_Be_Harvested (Utilities|Struct|BreakStruct_Saved_Plants _array_element)) (.Is_Regrowing (Utilities|Struct|BreakStruct_Saved_Plants _array_element)) (.Is_Destructed (Utilities|Struct|BreakStruct_Saved_Plants _array_element)) (.CurrentdurabilityFarmable (Utilities|Struct|BreakStruct_Saved_Plants _array_element)) (.GUID_Farmable (Utilities|Struct|BreakStruct_Saved_Plants _array_element)) (.Current_Decay_Time (Utilities|Struct|BreakStruct_Saved_Plants _array_element)) (.CurrentAmountofFertilizer (Utilities|Struct|BreakStruct_Saved_Plants _array_element)) (.CurrentAmountofWater (Utilities|Struct|BreakStruct_Saved_Plants _array_element)) (.Is_Decayed (Utilities|Struct|BreakStruct_Saved_Plants _array_element)) (.Is_Sick (Utilities|Struct|BreakStruct_Saved_Plants _array_element)) (.Is_Decaying (Utilities|Struct|BreakStruct_Saved_Plants _array_element)) (.FertilizerConsumed (Utilities|Struct|BreakStruct_Saved_Plants _array_element)) (.LinkedPluckableYield (Utilities|Struct|BreakStruct_Saved_Plants _array_element)) true (.IsManuallyplacedinworld (Utilities|Struct|BreakStruct_Saved_Plants _array_element)) false true 0))
        (Utilities|Map|Add (LocalVariables|GetLocal_GUID_To_Actor) (.GUID_Farmable (Utilities|Struct|BreakStruct_Saved_Plants _array_element)) _returnvalue_3)
        (Utilities|Array|Add (LocalVariables|GetLocal%20%20Spawned%20Plants) _returnvalue_3)))
    (for _array_element_2 (LocalVariables|GetLocal%20%20Spawned%20Plants)
      (for _array_element_3 (Variables|/Game/FarmingSystem/Blueprints/Masters/BP_Farming_Master.BP_Farming_Master_C|GetLinked_Pluckable_Yield_GUIDS _array_element_2)
        (if (.ReturnValue (Utilities|Map|Find (LocalVariables|GetLocal_GUID_To_Actor) _array_element_3))
          (Utilities|Array|Add (Variables|/Game/FarmingSystem/Blueprints/Masters/BP_Farming_Master.BP_Farming_Master_C|GetLinked_Pluckable_Yield _array_element_2) (.Value (Utilities|Map|Find (LocalVariables|GetLocal_GUID_To_Actor) _array_element_3))))))))

(fn OnRepCurrentEquipedMesh
  (bind _current__equiped_mesh (Variables|Default|GetCurrent%20%20Equiped%20Mesh))
  (Utilities|IsValid (Variables|Default|GetCurrent%20%20Equiped%20Mesh)
    (:Is%20Valid
      (Utilities|IsValid (Variables|Default|GetCurrent_Attached_Actor)
        (:Is%20Valid
          (Actor|DestroyActor (Variables|Default|GetCurrent_Attached_Actor)))
        (:Is%20Not%20Valid
          _))
      (bind _returnvalue (Game|SpawnActorfromClass "/Game/FarmingSystem/Character/Blueprints/BP_Dummy_Equipment.BP_Dummy_Equipment_C" (Math|Transform|MakeTransform "0, 0, 0" "0, 0, 0" "1,1,1") "Undefined" 0 _current__equiped_mesh 0))
      (Transformation|AttachComponentToComponent _returnvalue (Variables|/Script/Engine.Character|GetMesh (Variables|Default|GetOwning%20character%20referemce)) (select (== _current__equiped_mesh "/Game/ResourcePack/Props/Basket/Mesh/SM_Basket_Small.SM_Basket_Small") "Hand_l" "Primary Weapon") "SnapToTarget" "SnapToTarget" "SnapToTarget" true)
      (Variables|Default|SetCurrent_Attached_Actor _returnvalue))
    (:Is%20Not%20Valid
      (Utilities|IsValid (Variables|Default|GetCurrent_Attached_Actor)
        (:Is%20Valid
          (Actor|DestroyActor (Variables|Default|GetCurrent_Attached_Actor)))))))

(fn OnRepAmountOfAnimationsPlayed
  (Class|AnimInstance|PlaySlotAnimationasDynamicMontage (Components|SkeletalMesh|GetAnimInstance (Variables|/Script/Engine.Character|GetMesh (Variables|Default|GetOwning%20character%20referemce))) (Variables|Default|GetAnimation%20To%20Play) "DefaultSlot" 0.25 0.25 1.0 1 -1.0 0.0))